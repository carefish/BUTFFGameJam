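; Obstacle spawner actor that places random obstacles at random spawn points during play.
; BeginPlay starts a timeline whose event track, Gibsumobstaklz, triggers each spawn.
; Every trigger independently picks a class from AvailableObstacles and a location from ObstacleSpawnpoints, then spawns that actor.
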(event `self.ReceiveBeginPlay`
  (bind _obstaclespawnpoints (`self.ObstacleSpawnpoints`))
  (bind _availableobstacles (`self.AvailableObstacles`))
  (`Timeline|Timeline_0`
    (:`gibsumobstaklz`
      (`|SpawnActorFromClass` (`KismetArrayLibrary.Array_Get` _availableobstacles (`KismetMathLibrary.RandomIntegerInRange` 0 (- (`KismetArrayLibrary.Array_Length` _availableobstacles) 1))) (`KismetMathLibrary.MakeTransform` (`KismetArrayLibrary.Array_Get` _obstaclespawnpoints (`KismetMathLibrary.RandomIntegerInRange` 0 (- (`KismetArrayLibrary.Array_Length` _obstaclespawnpoints) 1)))) "Undefined" "OverrideRootScale"))))

(fn `UserConstructionScript`)