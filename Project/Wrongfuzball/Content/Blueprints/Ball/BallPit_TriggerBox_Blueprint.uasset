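; Ball pit trigger box that sends any overlapping actor tagged "Ball" back to a random spawn point.
; On BeginPlay it caches every actor tagged "BallSpawnpoint" in an array.
; On overlap it moves the ball to a randomly indexed spawn point's location without sweep.
; The inclusive random range runs up to the array length, so it can pick an index one past the last spawn point.
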(event `self.ReceiveBeginPlay`
  (bind _outactors (`GameplayStatics.GetAllActorsWithTag` "BallSpawnpoint"))
  (set `self.BallSpawnpoints` _outactors))

(event `self.ReceiveActorBeginOverlap`
  (params (OtherActor :type "Actor Object Reference"))
  (bind _ballspawnpoints (`self.BallSpawnpoints`))
  (if (`self.ActorHasTag` OtherActor "Ball")
    (`self.K2_SetActorLocation` OtherActor (`self.K2_GetActorLocation` (`KismetArrayLibrary.Array_Get` _ballspawnpoints (`KismetMathLibrary.RandomIntegerInRange` 0 (`KismetArrayLibrary.Array_Length` _ballspawnpoints)))) false false)))

(fn `UserConstructionScript`)