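; Powerup spawner actor that spawns random powerups at random spawnpoints during play.
; A timeline started on BeginPlay fires an event track, each firing picking a random class from AvailablePowerups and a random entry from PowerupSpawnpoints.
; Each spawn copies WillSpawnAntiPowerup into its IsAntiPowerup flag.
; SpawnAntiPowerups switches that flag on, and the node that would clear it is unconnected, so it stays on.
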(event `self.ReceiveBeginPlay`
  (bind _availablepowerups (`self.AvailablePowerups`))
  (bind _powerupspawnpoints (`self.PowerupSpawnpoints`))
  (`Timeline|Timeline_0`
    (:`moarpowerupz`
      (bind _returnvalue (`|SpawnActorFromClass` (`KismetArrayLibrary.Array_Get` _availablepowerups (`KismetMathLibrary.RandomIntegerInRange` 0 (- (`KismetArrayLibrary.Array_Length` _availablepowerups) 1))) (`KismetMathLibrary.MakeTransform` (`KismetArrayLibrary.Array_Get` _powerupspawnpoints (`KismetMathLibrary.RandomIntegerInRange` 0 (- (`KismetArrayLibrary.Array_Length` _powerupspawnpoints) 1)))) "Undefined" "OverrideRootScale"))
      (set `/Game/Blueprints/Powerups/PowerupBase.IsAntiPowerup` (`self.WillSpawnAntiPowerup`) _returnvalue))))

(event `SpawnAntiPowerups`
  (set `self.WillSpawnAntiPowerup` true))

(fn `UserConstructionScript`)