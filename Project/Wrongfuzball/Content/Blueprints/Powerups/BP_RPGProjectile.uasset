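; RPG rocket projectile powerup actor that explodes on overlap and launches characters into the air.
; BeginPlay plays the flight sound at world origin.
; Both Sphere and ProjectileTriggerVolume overlaps ignore MyOwner and spawn explosion effects, at the hit actor and the projectile respectively.
; After a short delay, a hit Character is launched upward and the rocket is destroyed; non-Character hits leave it alive.
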(event `self.ReceiveBeginPlay`
  (`GameplayStatics.PlaySoundAtLocation` "/Game/Effects/Audio/SFX_RocketFlying.SFX_RocketFlying"))

(event `self.Sphere.OnComponentBeginOverlap`
  (params (OverlappedComponent :type "PrimitiveComponent Object Reference") (OtherActor :type "Actor Object Reference") (OtherComp :type "PrimitiveComponent Object Reference") (OtherBodyIndex :type Integer) (bFromSweep :type Boolean) (SweepResult :type "HitResult Structure (by ref)"))
  (bind _returnvalue (`self.K2_GetActorLocation` OtherActor))
  (if (!= OtherActor (`self.MyOwner`))
    ;[1 1 1] Projectile hits player
    (`GameplayStatics.SpawnSoundAtLocation` "/Game/Effects/Audio/SFX_RocketExplosion.SFX_RocketExplosion" _returnvalue)
    (`GameplayStatics.SpawnEmitterAtLocation` "/Game/StarterContent/Particles/P_Explosion.P_Explosion" _returnvalue)
    (`KismetSystemLibrary.Delay` 0.4)
    (bind _ascharacter (cast `Character` OtherActor))
    (`Character.LaunchCharacter` _ascharacter (0.0 0.0 800.0) false false)
    (`self.K2_DestroyActor`)))

(event `self.ProjectileTriggerVolume.OnComponentBeginOverlap`
  (params (OverlappedComponent :type "PrimitiveComponent Object Reference") (OtherActor :type "Actor Object Reference") (OtherComp :type "PrimitiveComponent Object Reference") (OtherBodyIndex :type Integer) (bFromSweep :type Boolean) (SweepResult :type "HitResult Structure (by ref)"))
  (bind _returnvalue (`self.K2_GetActorLocation`))
  (if (!= OtherActor (`self.MyOwner`))
    ;[1 1 1] Projectile hits player
    (`GameplayStatics.SpawnSoundAtLocation` "/Game/Effects/Audio/SFX_RocketExplosion.SFX_RocketExplosion" _returnvalue)
    (`GameplayStatics.SpawnEmitterAtLocation` "/Game/StarterContent/Particles/P_Explosion.P_Explosion" _returnvalue)
    (`KismetSystemLibrary.Delay` 0.4)
    (bind _ascharacter (cast `Character` OtherActor))
    (`Character.LaunchCharacter` _ascharacter (0.0 0.0 800.0) false false)
    (`self.K2_DestroyActor`)))

(fn `UserConstructionScript`)